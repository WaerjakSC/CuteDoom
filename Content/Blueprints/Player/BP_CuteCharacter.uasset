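; Prototype player character Blueprint with placeholder weapon and health logic, much of it marked for a move to C++.
; R starts a delayed reload that does no ammo transfer and always takes the Glock branch, and 1 sets the gun type.
; G and H test damage and healing, with health resetting to max on death.
; Kick animation, multi-trace shotgun fire, spare-ammo checks and meat-pickup speed boost are disconnected and never run.
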(event `Key|R`
  (params (Key :type "Key Structure"))
  ;[1 1 1] TODO - Add checks for ammo and do all that stuff in C++
  (:`Pressed`
    (set `self.Reloading` true)
    (if true
      (if (`self.haveSpareGlockAmmo`)
        (`KismetSystemLibrary.Delay` 2.0)
        (`|ExecutionSequence`))
      (elif (`self.haveSpareShotgunAmmo`)
        (`KismetSystemLibrary.Delay` 3.0)
        (`|ExecutionSequence`)
        (else
          (`KismetSystemLibrary.PrintString` "You do not have enough Ammo to reload!"))))))

(event `Key|One`
  (params (Key :type "Key Structure"))
  ;[1 1 1] TODO - Weapon Swapping in C++
  (:`Pressed`
    (`|ExecutionSequence`
      (:`then_1`
        (set `self.gunType` 1)))))

(event `Key|G`
  (params (Key :type "Key Structure"))
  ;[1 1 1] Test for damage and healing
  (:`Pressed`
    (`self.Health_Deplete`)))

(event `Key|H`
  (params (Key :type "Key Structure"))
  ;[1 1 1] Test for damage and healing
  (:`Pressed`
    (`self.Health_Regen`)))

(event `self.ReceiveTick`
  (params (DeltaSeconds :type "Float (single-precision)"))
  ;[1 1 1] TODO - Function call when "Meat" object is picked up by player to increment and check if a certain amount has been collected.
)

(fn `Health_Deplete`
  (bind _output_get (set `self.Health` (- (`self.Health`) 20.0)))
  ;[1 1 1] reset health after death just for prototype
  (if (<= _output_get 0.0)
    (set `self.Health` (`self.MaxHealth`))))

(fn `Health_Regen`
  (set `self.Health` (+ (`self.Health`) 20.0)))

(fn `UserConstructionScript`)